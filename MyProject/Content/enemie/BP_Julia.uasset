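; BP_Julia is an AI enemy that chases the player and registers with the third-person game mode's living-enemy count.
; While alive, it issues AIMoveTo every tick with the player as target actor, alongside a random search location.
; AI perception records player sightings and holds DoOnce-gated logic for picking search points.
; Lethal damage turns it into a ragdoll, decrements the count and triggers the game mode's remaining-enemy check.
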(event `self.ReceiveAnyDamage`
  (params (Damage :type "Float (single-precision)") (DamageType :type "DamageType Object Reference") (InstigatedBy :type "Controller Object Reference") (DamageCauser :type "Actor Object Reference"))
  ;[1 1 1] prise de damage
  (if (not (`self.isDead`))
    (bind _output_get (set `self.Health` (- (`self.Health`) Damage)))
    (if (<= _output_get 0.0)
      (`CharacterMovementComponent.DisableMovement` (`self.CharacterMovement`))
      (`PrimitiveComponent.SetCollisionEnabled` (`self.CapsuleComponent`) "NoCollision")
      (`PrimitiveComponent.SetSimulatePhysics` (`self.Mesh`) true)
      (set `self.isDead` true)
      (bind _asbp_third_person_game_mode (cast `/Game/ThirdPerson/Blueprints/BP_ThirdPersonGameMode` (`GameplayStatics.GetGameMode`)))
      (`/Engine/EditorBlueprintResources/StandardMacros.DecrementInt` (`/Game/ThirdPerson/Blueprints/BP_ThirdPersonGameMode.EnemyAlive` _asbp_third_person_game_mode)
        (:`  `
          (`/Game/ThirdPerson/Blueprints/BP_ThirdPersonGameMode.CheckEnemyLeft` _asbp_third_person_game_mode))))))

(event `self.ReceiveTick`
  (params (DeltaSeconds :type "Float (single-precision)"))
  ;[1 1 1] AI
  (if (not (`self.isDead`))
    (`self.RunToThePlayer`)))

(event `self.ReceiveBeginPlay`
  ;[1 1 1] AI
  (bind _asbp_third_person_game_mode (cast `/Game/ThirdPerson/Blueprints/BP_ThirdPersonGameMode` (`GameplayStatics.GetGameMode`)))
  (`/Engine/EditorBlueprintResources/StandardMacros.IncrementInt` (`/Game/ThirdPerson/Blueprints/BP_ThirdPersonGameMode.EnemyAlive` _asbp_third_person_game_mode)
    (:`  `
      (bind _randomlocation (`NavigationSystemV1.K2_GetRandomLocationInNavigableRadius` (`self.K2_GetActorLocation`) 5000.0 null null))
      (set `self.LocationToSearch` _randomlocation)
      (bind _asbp_third_person_character (cast `/Game/ThirdPerson/Blueprints/BP_ThirdPersonCharacter` (`GameplayStatics.GetPlayerCharacter` 0)))
      (set `self.PlayerRef` _asbp_third_person_character))))

(event `RunToThePlayer`
  ;[1 1 1] AI
  (bind _asbp_third_person_character (cast `/Game/ThirdPerson/Blueprints/BP_ThirdPersonCharacter` (`GameplayStatics.GetPlayerCharacter` 0)))
  (`|AIMoveTo` self (`self.LocationToSearch`) _asbp_third_person_character 40.0
    (:`then`
      (`self.ResetChooseRandomLocToSearchThePlayer`)
      (`KismetSystemLibrary.Delay` 0.2)
      (`self.ChooseRandomLocToSearchThePlayer`))))

(event `self.AIPerception.OnTargetPerceptionUpdated`
  (params (Actor :type "Actor Object Reference") (Stimulus :type "AIStimulus Structure"))
  ;[1 1 1] AI
  (if true
    (bind _asbp_third_person_character (cast `/Game/ThirdPerson/Blueprints/BP_ThirdPersonCharacter` Actor))
    (set `self.PlayerRef` _asbp_third_person_character)
    (set `self.PlayerLocation` Stimulus_StimulusLocation)
    (set `self.CanSeeThePlayer` true)
    (else
      (set `self.LastPlayerLocation` Stimulus_StimulusLocation)
      (set `self.CanSeeThePlayer` false)
      (`/Engine/EditorBlueprintResources/StandardMacros.DoOnce` false :!label _label
        (:`Completed`
          (bind _randomlocation (`NavigationSystemV1.K2_GetRandomLocationInNavigableRadius` (`self.LastPlayerLocation`) 1000.0 null null))
          (set `self.LocationToSearch` _randomlocation))))))

(event `ChooseRandomLocToSearchThePlayer`
  ;[1 1 1] AI
  (goto _label))

(event `ResetChooseRandomLocToSearchThePlayer`
  ;[1 1 1] AI
  (goto _label :!via `Reset`))

(fn `Death`
  (`self.K2_DestroyActor`))

(fn `UserConstructionScript`)