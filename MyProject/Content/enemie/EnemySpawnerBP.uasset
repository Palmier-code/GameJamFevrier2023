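; Enemy spawner actor that spawns growing batches of BP_Julia enemies at its own transform.
; On BeginPlay it binds SpawnEnemy to the RespawnEnemy event of BP_ThirdPersonGameMode.
; Each call spawns a batch, nudging positions to avoid collisions but always spawning.
; It then raises the increment by one and adds it to the batch count, so waves grow at an accelerating rate.
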(event `self.ReceiveBeginPlay`
  (bind _asbp_third_person_game_mode (cast `/Game/ThirdPerson/Blueprints/BP_ThirdPersonGameMode` (`GameplayStatics.GetGameMode`)))
  (add `/Game/ThirdPerson/Blueprints/BP_ThirdPersonGameMode.RespawnEnemy` _asbp_third_person_game_mode (delegate `SpawnEnemy`)))

(event `SpawnEnemy`
  (for _ (range (+ (`self.EnemySpawned`) 1))
    (`|SpawnActorFromClass` "/Game/enemie/BP_Julia.BP_Julia_C" (`self.GetTransform`) "AdjustIfPossibleButAlwaysSpawn" "OverrideRootScale" null null))
  (`/Engine/EditorBlueprintResources/StandardMacros.IncrementInt` (`self.SpawnIncrement`)
    (:`  `
      (set `self.EnemySpawned` (+ (`self.EnemySpawned`) (`self.SpawnIncrement`))))))

(fn `UserConstructionScript`)